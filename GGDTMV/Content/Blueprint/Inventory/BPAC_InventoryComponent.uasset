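; BPAC_InventoryComponent is an actor component that holds an inventory as an array of slots.
; On BeginPlay it fills the slot array with a configurable number of entries, each flagged true and tagged with its index.
; AddItem takes an item ID and amount but only prints a debug message, without changing the slots.
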(event EventBeginPlay
  ;[0.15 0.15 0.15 0.5] Init number of inventory slots
  (CallFunction|InitializeInventory))

(event EventTick
  (params (DeltaSeconds :type Float%20%28single-precision%29)))

(fn InitializeInventory
  ;[0.15 0.15 0.15 0.5] That function Init inventory slots number
  (for _index (range 0 (- (Variables|Default|GetNum%20Inventory%20Slot) 1))
    (Utilities|Array|Add (Variables|Default|GetInventory%20Slot) (Utilities|Struct|MakeStruct_InventorySlotData true "(ItemID_4_AC16A4064E020BC02C021B862692314F=\"\",ItemCategory_25_5EAD0B3542D4479EAE5D898FCEC13BB6=NewEnumerator0,ItemName_9_B9A1FFB0436E2108168C519CDC65B72E=\"\",ItemDescription_11_02868DD2420D90ABC770D29929734B0E=\"\",EnergyOutput_28_7F8510644AEC8F19D31D0C92C9BE6BEC=0,Stability_30_59671C654A2CF0C0266D909CF5CBC63F=0,Efficency_32_ADEBB57E42507453342591A19A194409=0,CurrentQuantity_17_D538B63C42C40AD63C0F0D9AB8A0AB79=0,MaxQuantity_18_C240A1FE4833DADF1F5E70A3D49A0D3F=0,ItemIcon_21_4040111144DA7BC838E8279384675146=None,ItemBPClass_24_258AEF5D4F34BAC0508EE3AEBA0B9698=None)" _index))))

(fn AddItem
  (params (Item%20ID :type String) (Amount :type Integer))
  (Development|PrintString (Utilities|String|Append (Utilities|String|ToString(Integer) Amount) " " Item%20ID " Added to inventory!")))